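; StateBlock_Subject is an event block sprite actor that represents a school subject state: none, Korean, English or Math.
; On BeginPlay it resets to NONE through SetMySprite.
; SetMySprite stores the subject, swaps the render component's sprite, and rewrites the actor tags with StateBlock, Subject and a subject-specific tag.
; Click and overlap handlers are present but perform no actions.
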(event `self.ReceiveBeginPlay`
  (`self.SetMySprite` "NewEnumerator3"))

(event `self.RenderComponent.OnClicked`
  (params (TouchedComponent :type "PrimitiveComponent Object Reference") (ButtonPressed :type "Key Structure")))

(event `self.ReceiveActorBeginOverlap`
  (params (OtherActor :type "Actor Object Reference")))

(event `self.ReceiveTick`
  (params (DeltaSeconds :type "Float (single-precision)")))

(event `self.ReceiveActorEndOverlap`
  (params (OtherActor :type "Actor Object Reference"))
  (if (`KismetArrayLibrary.Array_Contains` (`Actor.Tags` OtherActor) "PLAYER")
    _))

(fn `SetMySprite`
  (params (NewSprite :type "/Game/Blueprint/EventBlock/Subject_State_Enum Enum" :default "NewEnumerator0"))
  (bind _output_get (set `self.EventBlockSubjectState` NewSprite))
  (`PaperSpriteComponent.SetSprite` (`self.RenderComponent`) (select `/Game/Blueprint/EventBlock/Subject_State_Enum` (`self.EventBlockSubjectState`) :`NewEnumerator3` "/Game/Resources/NEW/Resources/UI/uisprite/user2_Sprite_7.user2_Sprite_7" :`NewEnumerator0` "/Game/Resources/NEW/Resources/Tileset/blockicon/korean.korean" :`NewEnumerator1` "/Game/Resources/NEW/Resources/Tileset/blockicon/english.english" :`NewEnumerator2` "/Game/Resources/NEW/Resources/Tileset/blockicon/math.math" :!type "PaperSprite Object Reference"))
  (set `self.Tags` (`|MakeArray` "StateBlock" "Subject" (select `/Game/Blueprint/EventBlock/Subject_State_Enum` _output_get :`NewEnumerator3` "NONESUBJECT" :`NewEnumerator0` "KOREAN" :`NewEnumerator1` "ENGLISH" :`NewEnumerator2` "MATH" :!type "Name")))
  (return))

(fn `UserConstructionScript`)