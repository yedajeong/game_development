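; EventBlock is a clickable event tile that holds a base activity, subject and study method, shown as three side-by-side sprite blocks spawned on BeginPlay.
; Clicking it while accessible applies the player's selected states, updating the sprites and rebuilding the actor's tags from those enums.
; Overlap by a player tagged SICK forces the tile to Cure and locks it, darkening all three sprites.
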(event `self.ReceiveBeginPlay`
  (`self.InitializeStateBlock`)
  (bind _asplayer_blueprint (cast `/Game/Blueprint/Player_Blueprint` (`GameplayStatics.GetPlayerCharacter` 0)))
  (set `self.MyCharacter` _asplayer_blueprint))

(event `self.RenderComponent.OnClicked`
  (params (TouchedComponent :type "PrimitiveComponent Object Reference") (ButtonPressed :type "Key Structure"))
  (bind _mycharacter (`self.MyCharacter`))
  (`GameplayStatics.PlaySound2D` "/Game/Resources/Sound/click_003.click_003" 1.0 1.0 0.0 null null)
  (if (`self.EventBlockAceesibleState`)
    (`self.SetStateBlockState` (`/Game/Blueprint/Player_Blueprint.SelectedBaseStateEnum` _mycharacter) (`/Game/Blueprint/Player_Blueprint.SelectedSubjectStateEnum` _mycharacter) (`/Game/Blueprint/Player_Blueprint.SelectedMethodStateEnum` _mycharacter))))

(event `self.ReceiveActorBeginOverlap`
  (params (OtherActor :type "Actor Object Reference"))
  (bind _tags (`Actor.Tags` OtherActor))
  (if (and (`KismetArrayLibrary.Array_Contains` _tags "PLAYER") (`KismetArrayLibrary.Array_Contains` _tags "SICK"))
    (`self.SetStateBlockState` "NewEnumerator2")
    (`self.SetBlockAcessibility` false)))

(event `self.ReceiveTick`
  (params (DeltaSeconds :type "Float (single-precision)")))

(event `self.ReceiveActorEndOverlap`
  (params (OtherActor :type "Actor Object Reference"))
  (if (`KismetArrayLibrary.Array_Contains` (`Actor.Tags` OtherActor) "PLAYER")
    _))

(fn `InitializeStateBlock`
  (locals (NewLocalVar_0 :type "/Game/Blueprint/EventBlock/StateBlock_Method Class Reference" :default "BlueprintGeneratedClass'/Game/Blueprint/EventBlock/StateBlock_Method.StateBlock_Method_C'"))
  (bind _x (.x (.location (`self.GetTransform`))))
  (bind _z (.z (.location (`self.GetTransform`))))
  (bind _returnvalue (`|SpawnActorFromClass` "/Game/Blueprint/EventBlock/StateBlock_Base.StateBlock_Base_C" (`KismetMathLibrary.MakeTransform` (`KismetMathLibrary.MakeVector` (- _x 32.0) 0.5 _z)) "Undefined" "OverrideRootScale" null null)) ; Base 블록 생성
  (set `self.StateBlockBase` _returnvalue)
  (bind _returnvalue_2 (`|SpawnActorFromClass` "/Game/Blueprint/EventBlock/StateBlock_Subject.StateBlock_Subject_C" (`KismetMathLibrary.MakeTransform` (`KismetMathLibrary.MakeVector` _x 0.5 _z)) "Undefined" "OverrideRootScale" null null)) ; Subject 블록 생성
  (set `self.StateBlockSubject` _returnvalue_2)
  (bind _returnvalue_3 (`|SpawnActorFromClass` "/Game/Blueprint/EventBlock/StateBlock_Method.StateBlock_Method_C" (`KismetMathLibrary.MakeTransform` (`KismetMathLibrary.MakeVector` (+ _x 32.0) 0.5 _z)) "Undefined" "OverrideRootScale" null null)) ; Method 블록 생성
  (set `self.StateBlockMethod` _returnvalue_3))

(fn `SetBlockAcessibility`
  (params (MakeAcessible :type Boolean))
  (if MakeAcessible
    (`PaperSpriteComponent.SetSpriteColor` (`PaperSpriteActor.RenderComponent` (`self.StateBlockBase`)) (struct :`R` 1.0 :`G` 1.0 :`B` 1.0 :`A` 1.0))
    (`PaperSpriteComponent.SetSpriteColor` (`PaperSpriteActor.RenderComponent` (`self.StateBlockSubject`)) (struct :`R` 1.0 :`G` 1.0 :`B` 1.0 :`A` 1.0))
    (`PaperSpriteComponent.SetSpriteColor` (`PaperSpriteActor.RenderComponent` (`self.StateBlockMethod`)) (struct :`R` 1.0 :`G` 1.0 :`B` 1.0 :`A` 1.0))
    (set `self.EventBlockAceesibleState` true)
    (else
      (`PaperSpriteComponent.SetSpriteColor` (`PaperSpriteActor.RenderComponent` (`self.StateBlockBase`)) (struct :`R` 0.151042 :`G` 0.151042 :`B` 0.151042 :`A` 1.0))
      (`PaperSpriteComponent.SetSpriteColor` (`PaperSpriteActor.RenderComponent` (`self.StateBlockSubject`)) (struct :`R` 0.151042 :`G` 0.151042 :`B` 0.151042 :`A` 1.0))
      (`PaperSpriteComponent.SetSpriteColor` (`PaperSpriteActor.RenderComponent` (`self.StateBlockMethod`)) (struct :`R` 0.151042 :`G` 0.151042 :`B` 0.151042 :`A` 1.0))
      (set `self.EventBlockAceesibleState` false))))

(fn `SetStateBlockState`
  (params (BaseState :type "/Game/Blueprint/EventBlock/EventBlock_Base_State_Enum Enum" :default "NewEnumerator0") (SubjectState :type "/Game/Blueprint/EventBlock/Subject_State_Enum Enum" :default "NewEnumerator3") (MethodState :type "/Game/Blueprint/EventBlock/EventBlock_Method_State_Enum Enum" :default "NewEnumerator2"))
  (bind _output_get (set `self.EventBlockBaseState` BaseState))
  (bind _output_get_2 (set `self.EventBlockSubjectState` SubjectState))
  (bind _output_get_3 (set `self.EventBlockMethodState` MethodState))
  (set `self.Tags` (`|MakeArray` "EventBlock" (select `/Game/Blueprint/EventBlock/EventBlock_Base_State_Enum` _output_get :`NewEnumerator0` "REST" :`NewEnumerator1` "STUDY" :`NewEnumerator2` "CURE" :`NewEnumerator3` "TEST" :`NewEnumerator4` "TELEPORT" :!type "Name") (select `/Game/Blueprint/EventBlock/Subject_State_Enum` _output_get_2 :`NewEnumerator3` "NONESUBJECT" :`NewEnumerator0` "KOREAN" :`NewEnumerator1` "ENGLISH" :`NewEnumerator2` "MATH" :!type "Name") (select `/Game/Blueprint/EventBlock/EventBlock_Method_State_Enum` _output_get_3 :`NewEnumerator2` "NONEMETHOD" :`NewEnumerator0` "SELFSTUDY" :`NewEnumerator1` "CLASSSTUDY" :!type "Name")))
  (`/Game/Blueprint/EventBlock/StateBlock_Base.SetMySprite` (`self.StateBlockBase`) _output_get)
  (`/Game/Blueprint/EventBlock/StateBlock_Subject.SetMySprite` (`self.StateBlockSubject`) _output_get_2)
  (`/Game/Blueprint/EventBlock/StateBlock_Method.SetMySprite` (`self.StateBlockMethod`) _output_get_3))

(fn `UserConstructionScript`)