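; An event block actor that represents a study method state: none, self study or class study.
; SetMySprite stores the state, swaps the sprite on its render component and rewrites the actor tags to StateBlock, Method and a state-specific tag.
; It resets to the none state on BeginPlay.
; The click, overlap and tick events have no logic, apart from an empty PLAYER tag check on end overlap.
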(event `self.ReceiveBeginPlay`
  (`self.SetMySprite` "NewEnumerator2"))

(event `self.RenderComponent.OnClicked`
  (params (TouchedComponent :type "PrimitiveComponent Object Reference") (ButtonPressed :type "Key Structure")))

(event `self.ReceiveActorBeginOverlap`
  (params (OtherActor :type "Actor Object Reference")))

(event `self.ReceiveTick`
  (params (DeltaSeconds :type "Float (single-precision)")))

(event `self.ReceiveActorEndOverlap`
  (params (OtherActor :type "Actor Object Reference"))
  (if (`KismetArrayLibrary.Array_Contains` (`Actor.Tags` OtherActor) "PLAYER")
    _))

(fn `SetMySprite`
  (params (NewSprite :type "/Game/Blueprint/EventBlock/EventBlock_Method_State_Enum Enum" :default "NewEnumerator0"))
  (bind _output_get (set `self.EventBlockMethodState` NewSprite))
  (`PaperSpriteComponent.SetSprite` (`self.RenderComponent`) (select `/Game/Blueprint/EventBlock/EventBlock_Method_State_Enum` (`self.EventBlockMethodState`) :`NewEnumerator2` "/Game/Resources/NEW/Resources/UI/uisprite/user2_Sprite_7.user2_Sprite_7" :`NewEnumerator0` "/Game/Resources/NEW/Resources/Tileset/blockicon/athome.athome" :`NewEnumerator1` "/Game/Resources/NEW/Resources/Tileset/blockicon/lecture.lecture" :!type "PaperSprite Object Reference"))
  (set `self.Tags` (`|MakeArray` "StateBlock" "Method" (select `/Game/Blueprint/EventBlock/EventBlock_Method_State_Enum` _output_get :`NewEnumerator2` "NONEMETHOD" :`NewEnumerator0` "SELFSTUDY" :`NewEnumerator1` "CLASSSTUDY" :!type "Name")))
  (return))

(fn `UserConstructionScript`)