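; StateBlock_Base is a Paper2D block actor that represents an event state: Rest, Study, Cure, Test or Teleport.
; SetMySprite stores the state, picks the matching sprite for RenderComponent and rebuilds the actor tags with a state name alongside StateBlock and Base.
; BeginPlay always initializes it to Rest.
; The click, tick and overlap events are empty stubs, including an end-overlap check for the player tag.
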(event `self.ReceiveBeginPlay`
  (`self.SetMySprite` "NewEnumerator0"))

(event `self.RenderComponent.OnClicked`
  (params (TouchedComponent :type "PrimitiveComponent Object Reference") (ButtonPressed :type "Key Structure")))

(event `self.ReceiveActorBeginOverlap`
  (params (OtherActor :type "Actor Object Reference")))

(event `self.ReceiveTick`
  (params (DeltaSeconds :type "Float (single-precision)")))

(event `self.ReceiveActorEndOverlap`
  (params (OtherActor :type "Actor Object Reference"))
  (if (`KismetArrayLibrary.Array_Contains` (`Actor.Tags` OtherActor) "PLAYER")
    _))

(fn `SetMySprite`
  (params (NewSprite :type "/Game/Blueprint/EventBlock/EventBlock_Base_State_Enum Enum" :default "NewEnumerator0"))
  (bind _output_get (set `self.EventBlockBaseState` NewSprite))
  (`PaperSpriteComponent.SetSprite` (`self.RenderComponent`) (select `/Game/Blueprint/EventBlock/EventBlock_Base_State_Enum` (`self.EventBlockBaseState`) :`NewEnumerator0` "/Game/Resources/NEW/Resources/Tileset/blockicon/rest.rest" :`NewEnumerator1` "/Game/Resources/NEW/Resources/Tileset/blockicon/study.study" :`NewEnumerator2` "/Game/Resources/NEW/Resources/Tileset/blockicon/heal.heal" :`NewEnumerator3` "/Game/Resources/Tileset/Event_Tileset_Sprite/Event_Tileset_Sprite_10.Event_Tileset_Sprite_10" :`NewEnumerator4` "/Game/Resources/NEW/Resources/Tileset/blockicon/unknown.unknown" :!type "PaperSprite Object Reference"))
  (set `self.Tags` (`|MakeArray` "StateBlock" "Base" (select `/Game/Blueprint/EventBlock/EventBlock_Base_State_Enum` _output_get :`NewEnumerator0` "REST" :`NewEnumerator1` "STUDY" :`NewEnumerator2` "CURE" :`NewEnumerator3` "TEST" :`NewEnumerator4` "TELEPORT" :!type "Name")))
  (return))

(fn `UserConstructionScript`)