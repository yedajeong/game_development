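; EventBlock_Spawner builds a 31-day calendar of event blocks on BeginPlay, starting on a random weekday offset.
; BlockGenerate lays days out in seven-column week rows, each with morning, afternoon and evening EventBlocks linked by TeleportBlocks.
; Weekday morning and afternoon blocks get a random subject and accessibility set to false.
; Each day's last teleport sprite differs at week's end, and an EndBlock follows the final day.
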(event `self.ReceiveBeginPlay`
  (`|ExecutionSequence`
    (:`then_0`
      (`self.DayVariableInitialization`) ; 랜덤으로 달력에 필요한 변수를 결정합니다.
    )
    (:`then_1`
      (`self.BlockGenerate`) ; 달력 변수들에 따라 이벤트블록을 생성합니다.
    )))

(fn `BlockGenerate`
  (locals (InitialLocation_X :type "Float (double-precision)" :default 0.0) (InitialLocation_Z :type "Float (double-precision)" :default 0.0) (NewLocalVar_0 :type Integer :default 0))
  (bind _returnvalue (mod (+ (`self.StartingDay`) (`self.CurrentDay`)) 7))
  (bind _returnvalue_2 (mod (+ (`self.StartingDay`) (`self.CurrentDay`)) 7))
  (bind _returnvalue_3 (`KismetMathLibrary.Conv_IntToDouble` (- -32 (* (`self.CurrentWeek`) 128))))
  (bind _returnvalue_4 (+ (`KismetMathLibrary.Conv_IntToDouble` (* (mod (+ (`self.StartingDay`) (`self.CurrentDay`)) 7) 96)) 32.0))
  (while (< (`self.CurrentDay`) (`self.DayRange`))
    (set `local.InitialLocation_X` _returnvalue_4)
    (set `local.InitialLocation_Z` _returnvalue_3)
    (bind _returnvalue_5 (`|SpawnActorFromClass` "/Game/Blueprint/EventBlock/EventBlock.EventBlock_C" (`KismetMathLibrary.MakeTransform` (`KismetMathLibrary.MakeVector` (`local.InitialLocation_X`) 1.0 (`local.InitialLocation_Z`))) "Undefined" "OverrideRootScale" null null)) ; 오전 EventBlock
    (if (and (!= _returnvalue_2 5) (!= _returnvalue_2 6))
      (`/Game/Blueprint/EventBlock/EventBlock.SetStateBlockState` _returnvalue_5 "NewEnumerator1" (select `int` (`KismetMathLibrary.RandomInteger` 3) :`0` "NewEnumerator0" :`1` "NewEnumerator1" :`2` "NewEnumerator2" :!type "/Game/Blueprint/EventBlock/Subject_State_Enum Enum") "NewEnumerator1")
      (`/Game/Blueprint/EventBlock/EventBlock.SetBlockAcessibility` _returnvalue_5 false))
    (bind _returnvalue_6 (`|SpawnActorFromClass` "/Game/Blueprint/EventBlock/TeleportBlock.TeleportBlock_C" (`KismetMathLibrary.MakeTransform` (`KismetMathLibrary.MakeVector` (+ (`local.InitialLocation_X`) 32.0) 0.0 (`local.InitialLocation_Z`))) "Undefined" "OverrideRootScale" null null)) ; 오전->오후TeleportBlock
    (`/Game/Blueprint/EventBlock/TeleportBlock.SetMySprite` _returnvalue_6 "NewEnumerator3")
    (bind _returnvalue_7 (`|SpawnActorFromClass` "/Game/Blueprint/EventBlock/EventBlock.EventBlock_C" (`KismetMathLibrary.MakeTransform` (`KismetMathLibrary.MakeVector` (`local.InitialLocation_X`) 1.0 (- (`local.InitialLocation_Z`) 32.0))) "Undefined" "OverrideRootScale" null null)) ; 오후  EventBlock
    (if (and (!= _returnvalue 5) (!= _returnvalue 6))
      (`/Game/Blueprint/EventBlock/EventBlock.SetStateBlockState` _returnvalue_7 "NewEnumerator1" (select `int` (`KismetMathLibrary.RandomInteger` 3) :`0` "NewEnumerator0" :`1` "NewEnumerator1" :`2` "NewEnumerator2" :!type "/Game/Blueprint/EventBlock/Subject_State_Enum Enum") "NewEnumerator1")
      (`/Game/Blueprint/EventBlock/EventBlock.SetBlockAcessibility` _returnvalue_7 false))
    (bind _returnvalue_8 (`|SpawnActorFromClass` "/Game/Blueprint/EventBlock/TeleportBlock.TeleportBlock_C" (`KismetMathLibrary.MakeTransform` (`KismetMathLibrary.MakeVector` (+ (`local.InitialLocation_X`) 32.0) 0.0 (- (`local.InitialLocation_Z`) 32.0))) "Undefined" "OverrideRootScale" null null)) ; 오후->저녁TeleportBlock
    (`/Game/Blueprint/EventBlock/TeleportBlock.SetMySprite` _returnvalue_8 "NewEnumerator3")
    (`|SpawnActorFromClass` "/Game/Blueprint/EventBlock/EventBlock.EventBlock_C" (`KismetMathLibrary.MakeTransform` (`KismetMathLibrary.MakeVector` (`local.InitialLocation_X`) 1.0 (- (`local.InitialLocation_Z`) 64.0))) "Undefined" "OverrideRootScale" null null) ; 저녁 EventBlock
    (bind _returnvalue_9 (`|SpawnActorFromClass` "/Game/Blueprint/EventBlock/TeleportBlock.TeleportBlock_C" (`KismetMathLibrary.MakeTransform` (`KismetMathLibrary.MakeVector` (+ (`local.InitialLocation_X`) 32.0) 0.0 (- (`local.InitialLocation_Z`) 64.0))) "Undefined" "OverrideRootScale" null null)) ; 일일TeleportBlock
    (if (== (mod (+ (`self.StartingDay`) (`self.CurrentDay`)) 7) 6)
      (`/Game/Blueprint/EventBlock/TeleportBlock.SetMySprite` _returnvalue_9 "NewEnumerator1")
      (else
        (`/Game/Blueprint/EventBlock/TeleportBlock.SetMySprite` _returnvalue_9 "NewEnumerator0")))
    (set `self.CurrentDay` (+ (`self.CurrentDay`) 1))
    (set `self.CurrentWeek` (/ (+ (`self.StartingDay`) (`self.CurrentDay`)) 7)))
  (set `local.InitialLocation_X` _returnvalue_4)
  (set `local.InitialLocation_Z` _returnvalue_3)
  (`|SpawnActorFromClass` "/Game/Blueprint/EventBlock/EndBlock.EndBlock_C" (`KismetMathLibrary.MakeTransform` (`KismetMathLibrary.MakeVector` (`local.InitialLocation_X`) 1.0 (`local.InitialLocation_Z`))) "Undefined" "OverrideRootScale" null null))

(fn `DayVariableInitialization`
  (set `self.StartingDay` (`KismetMathLibrary.RandomInteger` 6))
  (set `self.DayRange` 31)
  (set `self.EndingDay` (mod (+ (- (`self.StartingDay`) 1) (mod (`self.DayRange`) 7)) 7))
  (set `self.WeekRange` (`KismetMathLibrary.FCeil` (/ (`KismetMathLibrary.Conv_IntToDouble` (+ (`self.StartingDay`) (`self.DayRange`))) 7.0))))

(fn `UserConstructionScript`)