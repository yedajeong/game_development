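; Score_Manager tracks a score and level for each subject using map variables.
; ScoreUpdate rewrites a subject's score and calls LevelUpdate, which advances the level one enum step when the score exceeds that level's threshold.
; ScoreUpdate removes the map entry before Find reads it, so the stored score becomes just the new points instead of a running total.
; The event graph and construction script are empty.
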(fn `LevelUpdate`
  (params (SubjectToUpate :type "/Game/Blueprint/EventBlock/Subject_State_Enum Enum" :default "NewEnumerator3"))
  (locals (SubjectScore :type "Float (double-precision)") (SubjectLevel :type "/Game/Blueprint/EventBlock/Score_Level_Enum Enum" :default "NewEnumerator3") (SubjectTheshold :type "Float (double-precision)") (Subject :type "/Game/Blueprint/EventBlock/Subject_State_Enum Enum" :default "NewEnumerator3"))
  (set `local.Subject` SubjectToUpate)
  (set `local.SubjectScore` (`BlueprintMapLibrary.Map_Find` (`self.ScoreSubject`) (`local.Subject`)))
  (set `local.SubjectLevel` (`BlueprintMapLibrary.Map_Find` (`self.LevelSubject`) (`local.Subject`)))
  (set `local.SubjectTheshold` (`BlueprintMapLibrary.Map_Find` (`self.ThresholdLevel`) (`local.SubjectLevel`)))
  (if (> (`local.SubjectScore`) (`local.SubjectTheshold`))
    (`BlueprintMapLibrary.Map_Remove` (`self.LevelSubject`) (`local.Subject`))
    (if (`|EnumEquality` (`local.SubjectLevel`) "NewEnumerator0")
      (`BlueprintMapLibrary.Map_Add` (`self.LevelSubject`) (`local.Subject`) "NewEnumerator1")
      (elif (`|EnumEquality` (`local.SubjectLevel`) "NewEnumerator1")
        (`BlueprintMapLibrary.Map_Add` (`self.LevelSubject`) (`local.Subject`) "NewEnumerator2")
        (elif (`|EnumEquality` (`local.SubjectLevel`) "NewEnumerator2")
          (`BlueprintMapLibrary.Map_Add` (`self.LevelSubject`) (`local.Subject`) "NewEnumerator4"))))))

(fn `ScoreUpdate`
  (params (SubjectToUpdate :type "/Game/Blueprint/EventBlock/Subject_State_Enum Enum" :default "NewEnumerator3") (UpdatePoint :type "Float (double-precision)"))
  (bind _scoresubject (`self.ScoreSubject`))
  (`BlueprintMapLibrary.Map_Remove` _scoresubject SubjectToUpdate)
  (`BlueprintMapLibrary.Map_Add` _scoresubject SubjectToUpdate (+ UpdatePoint (`BlueprintMapLibrary.Map_Find` _scoresubject SubjectToUpdate)))
  (`self.LevelUpdate` SubjectToUpdate))

(fn `UserConstructionScript`)